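; Player pawn Blueprint that handles forward and backward movement input.
; The Bouger/Avant and Bouger/Arriere axis events each feed their value into AddMovementInput along a forward vector built from control-rotation yaw only, so pitch and roll do not affect direction.
; No strafing, look input or other gameplay logic is in the graphs; BeginPlay, overlap, Tick and construction are empty.
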(event `InputAxis|Bouger/Avant`
  (params (AxisValue :type "Float (single-precision)"))
  ;[1 1 1] avancer Avant/Arriere
  (`self.AddMovementInput` (`KismetMathLibrary.GetForwardVector` (`KismetMathLibrary.MakeRotator` 0.0 0.0 (.yaw (`self.GetControlRotation`)))) AxisValue))

(event `InputAxis|Bouger/Arriere`
  (params (AxisValue :type "Float (single-precision)"))
  ;[1 1 1] avancer Avant/Arriere
  (`self.AddMovementInput` (`KismetMathLibrary.GetForwardVector` (`KismetMathLibrary.MakeRotator` 0.0 0.0 (.yaw (`self.GetControlRotation`)))) AxisValue))

(fn `UserConstructionScript`)