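; BP_pion is a game piece that carries a team color: Blue Player, Red Player or Neutral.
; SetColor stores the color and sets the static mesh material's Color parameter to blue, red or yellow to match.
; RandomizeColor takes a player color and randomly passes either that color or Neutral to SetColor, with equal odds.
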(event `SetColor`
  (params (Color :type "/Game/PROJECT/Pions/E_PlayersColor Enum" :default "NewEnumerator0"))
  (bind _staticmesh (`self.StaticMesh`))
  (bind _output_get (set `self.Color` Color))
  (switch `/Game/PROJECT/Pions/E_PlayersColor` _output_get
    (:`NewEnumerator0`
      (`MeshComponent.SetVectorParameterValueOnMaterials` _staticmesh "Color" (0.0 0.0 1.0)))
    (:`NewEnumerator1`
      (`MeshComponent.SetVectorParameterValueOnMaterials` _staticmesh "Color" (1.0 0.0 0.0)))
    (:`NewEnumerator2`
      (`MeshComponent.SetVectorParameterValueOnMaterials` _staticmesh "Color" (1.0 1.0 0.0)))))

(event `Randomize Color`
  (params (Color :type "/Game/PROJECT/Pions/E_PlayersColor Enum" :default "NewEnumerator0"))
  (switch `/Game/PROJECT/Pions/E_PlayersColor` Color
    (:`NewEnumerator0`
      (`self.SetColor` (select `int` (`KismetMathLibrary.RandomIntegerInRange` 0 1) :`0` "NewEnumerator0" :`1` "NewEnumerator2" :!type "/Game/PROJECT/Pions/E_PlayersColor Enum")))
    (:`NewEnumerator1`
      (`self.SetColor` (select `int` (`KismetMathLibrary.RandomIntegerInRange` 0 1) :`0` "NewEnumerator1" :`1` "NewEnumerator2" :!type "/Game/PROJECT/Pions/E_PlayersColor Enum")))))

(fn `UserConstructionScript`)