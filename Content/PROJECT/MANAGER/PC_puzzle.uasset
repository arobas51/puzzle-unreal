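; Player controller for a two-player, turn-based grid puzzle, opening with music and a timed cinematic before showing the main menu widget.
; StartNewGame spawns colour-randomized pawns for Blue and Red, then a looping timer flips turns, resetting the chronometer and showing only the active side's pawns.
; Tick traces from the camera through the cursor to highlight the hovered BP_Grid square.
; Letter-number positions map to the product of both indices, so keys collide.
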(event `DistributePions`
  (bind _arrayofpionsplayerblue (`self.ArrayOfPionsPlayerBlue`))
  (bind _arrayofpionsplayerred (`self.ArrayOfPionsPlayerRed`))
  (for _index (range 5)
    (bind _returnvalue (`|SpawnActorFromClass` "/Game/PROJECT/Pions/BP_pion.BP_pion_C" (`KismetMathLibrary.MakeTransform` (0.0 0.0 0.0) (struct) (1.9 1.9 1.9)) "Undefined" "OverrideRootScale" null null))
    (`KismetArrayLibrary.Array_Add` (`self.ArrayOfPionsPlayerBlue`) _returnvalue)
    (`/Game/PROJECT/Pions/BP_pion.Randomize Color` _returnvalue "NewEnumerator0")
    (bind _returnvalue_2 (`GameplayStatics.GetActorOfClass` "/Game/PROJECT/GRID/BP_Grid.BP_Grid_C"))
    (bind _output (`|GetArrayItem` (`/Game/PROJECT/GRID/BP_Grid.squaresArray` _returnvalue_2) 99))
    (bind (_returnvalue_x _returnvalue_y _returnvalue_z) (`KismetMathLibrary.BreakVector` (`SceneComponent.K2_GetComponentLocation` _output)))
    (`self.K2_SetActorLocation` _returnvalue (`KismetMathLibrary.MakeVector` (+ _returnvalue_y (* (* _index (.x (`.BoxExtent` (`KismetSystemLibrary.GetComponentBounds` _output)))) 2.0) 800.0) 2400.0 _returnvalue_z) false false)
    (`self.SetActorHiddenInGame` _returnvalue true))
  (for _index_2 (range 5)
    (bind _returnvalue_3 (`|SpawnActorFromClass` "/Game/PROJECT/Pions/BP_pion.BP_pion_C" (`KismetMathLibrary.MakeTransform` (0.0 0.0 0.0) (struct) (1.9 1.9 1.9)) "Undefined" "OverrideRootScale" null null))
    (`KismetArrayLibrary.Array_Add` (`self.ArrayOfPionsPlayerRed`) _returnvalue_3)
    (`/Game/PROJECT/Pions/BP_pion.Randomize Color` _returnvalue_3 "NewEnumerator1")
    (bind _returnvalue_4 (`GameplayStatics.GetActorOfClass` "/Game/PROJECT/GRID/BP_Grid.BP_Grid_C"))
    (bind _output_2 (`|GetArrayItem` (`/Game/PROJECT/GRID/BP_Grid.squaresArray` _returnvalue_4) 99))
    (bind (_returnvalue_x_2 _returnvalue_y_2 _returnvalue_z_2) (`KismetMathLibrary.BreakVector` (`SceneComponent.K2_GetComponentLocation` _output_2)))
    (`self.K2_SetActorLocation` _returnvalue_3 (`KismetMathLibrary.MakeVector` (+ _returnvalue_y_2 (* (* _index_2 (.x (`.BoxExtent` (`KismetSystemLibrary.GetComponentBounds` _output_2)))) 2.0) 800.0) 2400.0 _returnvalue_z_2) false false)
    (`self.SetActorHiddenInGame` _returnvalue_3 true))
  (for _index_3 (range 5)
    (bind _returnvalue_5 (`|SpawnActorFromClass` "/Game/PROJECT/Pions/BP_pion.BP_pion_C" (`KismetMathLibrary.MakeTransform` (0.0 0.0 0.0) (struct) (1.9 1.9 1.9)) "Undefined" "OverrideRootScale" null null))
    (`KismetArrayLibrary.Array_Add` _arrayofpionsplayerblue _returnvalue_5)
    (`/Game/PROJECT/Pions/BP_pion.Randomize Color` _returnvalue_5 "NewEnumerator0")
    (bind (_returnvalue_x_3 _returnvalue_y_3 _returnvalue_z_3) (`KismetMathLibrary.BreakVector` (`self.K2_GetActorLocation` (`|GetArrayItem` _arrayofpionsplayerblue _index_3))))
    (`self.K2_SetActorLocation` _returnvalue_5 (`KismetMathLibrary.MakeVector` _returnvalue_x_3 (+ _returnvalue_y_3 400.0) _returnvalue_z_3) false false))
  (for _index_4 (range 5)
    (bind _returnvalue_6 (`|SpawnActorFromClass` "/Game/PROJECT/Pions/BP_pion.BP_pion_C" (`KismetMathLibrary.MakeTransform` (0.0 0.0 0.0) (struct) (1.9 1.9 1.9)) "Undefined" "OverrideRootScale" null null))
    (`KismetArrayLibrary.Array_Add` _arrayofpionsplayerred _returnvalue_6)
    (`/Game/PROJECT/Pions/BP_pion.Randomize Color` _returnvalue_6 "NewEnumerator1")
    (bind (_returnvalue_x_4 _returnvalue_y_4 _returnvalue_z_4) (`KismetMathLibrary.BreakVector` (`self.K2_GetActorLocation` (`|GetArrayItem` _arrayofpionsplayerred _index_4))))
    (`self.K2_SetActorLocation` _returnvalue_6 (`KismetMathLibrary.MakeVector` _returnvalue_x_4 (+ _returnvalue_y_4 400.0) _returnvalue_z_4) false false)))

(event `StartNewGame`
  (bind _returnvalue (`|CreateWidget` "/Game/PROJECT/UI/W_gameUI.W_gameUI_C"))
  (bind _output_get (set `self.gameUI` _returnvalue))
  (`UserWidget.AddToViewport` _output_get 0)
  (`/Game/PROJECT/CHRONOMETER/BP_chronometer.SetTimeLimit` (`self.BP_chronometer`) 15.0)
  (`self.DistributePions`)
  (`KismetSystemLibrary.K2_SetTimer` null "FlipFlopPlayerTurn" 15.0 true)
  (`self.FlipFlopPlayerTurn`))

(event `FlipFlopPlayerTurn`
  (`/Game/PROJECT/CHRONOMETER/BP_chronometer.Reset` (`self.BP_chronometer`))
  (`/Engine/EditorBlueprintResources/StandardMacros.FlipFlop`
    (:`A`
      (`self.PlayerTurn` "NewEnumerator0")
      (set `self.currentColorTurn` "NewEnumerator0"))
    (:`B`
      (`self.PlayerTurn` "NewEnumerator1")
      (set `self.currentColorTurn` "NewEnumerator1"))))

(event `PlayerTurn`
  (params (playerNumber :type "/Game/PROJECT/Pions/E_PlayersColor Enum" :default "NewEnumerator0"))
  (switch `/Game/PROJECT/Pions/E_PlayersColor` playerNumber
    (:`NewEnumerator0`
      (for _array_element (`self.ArrayOfPionsPlayerRed`)
        (`self.SetActorHiddenInGame` _array_element true))
      (for _array_element_2 (`self.ArrayOfPionsPlayerBlue`)
        (`self.SetActorHiddenInGame` _array_element_2 false)))
    (:`NewEnumerator1`
      (for _array_element_3 (`self.ArrayOfPionsPlayerBlue`)
        (`self.SetActorHiddenInGame` _array_element_3 true))
      (for _array_element_4 (`self.ArrayOfPionsPlayerRed`)
        (`self.SetActorHiddenInGame` _array_element_4 false)))))

(event `Key|LeftMouseButton`
  (params (Key :type "Key Structure"))
  (:`Pressed`
    (set `self.bShowMouseCursor` true)))

(event `self.ReceiveBeginPlay`
  (`GameplayStatics.PlaySound2D` "/Game/PROJECT/MUSIC/stoneTempleMusic.stoneTempleMusic" 1.0 1.0 0.0 null null)
  (bind (_outactor _returnvalue) (`LevelSequencePlayer.CreateLevelSequencePlayer` "/Game/PROJECT/Cinematics/NewLevelSequence.NewLevelSequence" (make `MovieSceneSequencePlaybackSettings` true (make `MovieSceneSequenceLoopCount` -1) 1.0 0.0 false false false false false false false true)))
  (`MovieSceneSequencePlayer.Play` _returnvalue)
  (bind _output_get (set `self.Out Actor` _outactor))
  (`KismetSystemLibrary.Delay` 10.0)
  (`MovieSceneSequencePlayer.Stop` (`LevelSequenceActor.SequencePlayer` _output_get))
  (bind _returnvalue_2 (`GameplayStatics.GetActorOfClass` "/Script/Engine.CameraActor"))
  (`self.SetViewTargetWithBlend` _returnvalue_2 1.0)
  (`KismetSystemLibrary.Delay` 1.0)
  (bind _returnvalue_3 (`|CreateWidget` "/Game/PROJECT/UI/W_main.W_main_C" (`GameplayStatics.GetPlayerController` 0)))
  (bind _output_get_2 (set `self.MainWidget` _returnvalue_3))
  (`WidgetBlueprintLibrary.SetInputMode_GameAndUIEx` self _output_get_2 "DoNotLock" false)
  (`UserWidget.AddToViewport` _output_get_2 0))

(event `self.ReceiveTick`
  (params (DeltaSeconds :type "Float (single-precision)"))
  (bind (_locationx _locationy) (`self.GetMousePosition`))
  (bind _returnvalue (`GameplayStatics.GetActorOfClass` "/Script/Engine.CameraActor"))
  (bind _returnvalue_2 (`self.K2_GetActorLocation` _returnvalue))
  (bind (_outhit _returnvalue_3) (`KismetSystemLibrary.LineTraceSingle` _returnvalue_2 (+ _returnvalue_2 (* (`.WorldDirection` (`self.DeprojectScreenPositionToWorld` _locationx _locationy)) 100000.0)) "TraceTypeQuery1" true))
  (if _returnvalue_3
    (bind _returnvalue_4 (`GameplayStatics.GetActorOfClass` "/Game/PROJECT/GRID/BP_Grid.BP_Grid_C"))
    (for _array_element (`/Game/PROJECT/GRID/BP_Grid.squaresArray` _returnvalue_4)
      (if (== _array_element (`.HitComponent` (`GameplayStatics.BreakHitResult` _outhit)))
        (`MeshComponent.SetVectorParameterValueOnMaterials` _array_element "Color Emissive" (1.0 0.0 0.0))
        (`MeshComponent.SetVectorParameterValueOnMaterials` _array_element "Color" (1.0 0.0 0.0))
        (set `self.HoveredSquare` _array_element)
        (else
          (`MeshComponent.SetVectorParameterValueOnMaterials` _array_element "Color Emissive" (1.0 1.0 1.0))
          (`MeshComponent.SetVectorParameterValueOnMaterials` _array_element "Color" (0.0 0.0 0.0)))))))

(fn `GetNumberByPosition`
  (params (NewParam :type "/Game/PROJECT/GRID/STR_position Structure"))
  (returns (ReturnValue :type Integer))
  (bind (_letter _number) (break `/Game/PROJECT/GRID/STR_position` NewParam))
  (return (* (select `/Game/PROJECT/GRID/E_PositionNumber` _number :`NewEnumerator0` 1 :`NewEnumerator1` 2 :`NewEnumerator2` 3 :`NewEnumerator3` 4 :`NewEnumerator4` 5 :`NewEnumerator5` 6 :`NewEnumerator6` 7 :`NewEnumerator7` 8 :`NewEnumerator8` 9 :`NewEnumerator9` 10) (select `/Game/PROJECT/GRID/E_PositionLetter` _letter :`NewEnumerator0` 1 :`NewEnumerator1` 2 :`NewEnumerator2` 3 :`NewEnumerator3` 4 :`NewEnumerator4` 5 :`NewEnumerator5` 6 :`NewEnumerator6` 7 :`NewEnumerator7` 8 :`NewEnumerator8` 9 :`NewEnumerator9` 10))))

(fn `GetPositionByNumber`
  (params (`Dimension 1` :type Integer))
  (returns (Output :type "/Game/PROJECT/GRID/STR_position Structure"))
  (bind _values (`BlueprintMapLibrary.Map_Values` (`self.PositionsByAbsoluteNumberArray`)))
  (return (`|GetArrayItem` _values `Dimension 1`)))

(fn `UserConstructionScript`
  (for _index (range 1 11)
    (for _index_2 (range 1 11)
      (`BlueprintMapLibrary.Map_Add` (`self.PositionsByAbsoluteNumberArray`) (* _index _index_2) (make `/Game/PROJECT/GRID/STR_position` (select `int` _index :`0` "NewEnumerator10" :`1` "NewEnumerator0" :`2` "NewEnumerator1" :`3` "NewEnumerator2" :`4` "NewEnumerator3" :`5` "NewEnumerator4" :`6` "NewEnumerator5" :`7` "NewEnumerator6" :`8` "NewEnumerator7" :`9` "NewEnumerator8" :`10` "NewEnumerator9" :!type "/Game/PROJECT/GRID/E_PositionLetter Enum") (select `int` _index_2 :`0` "NewEnumerator10" :`1` "NewEnumerator0" :`2` "NewEnumerator1" :`3` "NewEnumerator2" :`4` "NewEnumerator3" :`5` "NewEnumerator4" :`6` "NewEnumerator5" :`7` "NewEnumerator6" :`8` "NewEnumerator7" :`9` "NewEnumerator8" :`10` "NewEnumerator9" :!type "/Game/PROJECT/GRID/E_PositionNumber Enum"))))))