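; BP_chronometer is a pausable timer that tracks elapsed time against a time limit.
; Tick adds delta seconds to the current time unless paused, and Reset zeroes it.
; GetCurrentTime returns either the elapsed time or, in countdown mode, the limit minus elapsed.
; SetTimeLimit accepts only positive values, and nothing clamps the time or fires when the limit is reached.
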(event `Reset`
  (set `self.CurrentTime` 0.0)
  (`self.SetTimeLimit` (`self.timeLimit`)))

(event `Pause`
  (set `self.paused` true))

(event `UnPause`
  (set `self.paused` false))

(event `self.ReceiveTick`
  (params (DeltaSeconds :type "Float (single-precision)"))
  (if (not (`self.paused`))
    (set `self.CurrentTime` (+ DeltaSeconds (`self.CurrentTime`)))))

(event `SetTimeLimit`
  (params (A :type "Float (double-precision)"))
  (if (> A 0.0)
    (set `self.timeLimit` A)))

(fn `GetCurrentTime`
  (params (countdown :type Boolean))
  (returns (CurrentTime :type "Float (double-precision)"))
  (if countdown
    (return (- (`self.timeLimit`) (`self.CurrentTime`)))
    (else
      (return (`self.CurrentTime`)))))