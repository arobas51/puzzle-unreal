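; BP_Grid builds a board of BP_square tiles at BeginPlay, each with a letter and number index, attached and laid out around its root by mesh bounds.
; Neighbor lookups use offsets in the flat square array, assuming ten squares per letter index regardless of grid size variables.
; GetCrossedAdjacentPlaces returns orthogonal neighbors and their occupancy, trimming off-board squares only from the combined list.
; GetDirection converts two adjacent squares into a direction.
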(event `self.ReceiveBeginPlay`
  (for _index (range (`self.gridWidth`))
    (for _index_2 (range (`self.gridHeight`))
      (bind _returnvalue (`|SpawnActorFromClass` "/Game/PROJECT/GRID/BP_square.BP_square_C" (`KismetMathLibrary.MakeTransform` (0.0 0.0 0.0)) "Undefined" "OverrideRootScale" null null))
      (`KismetArrayLibrary.Array_Add` (`self.squaresArray`) _returnvalue)
      (set `/Game/PROJECT/GRID/BP_square.indexLetter` (select `int` _index :`0` "NewEnumerator0" :`1` "NewEnumerator1" :`2` "NewEnumerator2" :`3` "NewEnumerator3" :`4` "NewEnumerator4" :`5` "NewEnumerator5" :`6` "NewEnumerator6" :`7` "NewEnumerator7" :`8` "NewEnumerator8" :`9` "NewEnumerator9" :!type "/Game/PROJECT/GRID/E_PositionLetter Enum") _returnvalue)
      (set `/Game/PROJECT/GRID/BP_square.indexNumber` (select `int` _index_2 :`0` "NewEnumerator0" :`1` "NewEnumerator1" :`2` "NewEnumerator2" :`3` "NewEnumerator3" :`4` "NewEnumerator4" :`5` "NewEnumerator5" :`6` "NewEnumerator6" :`7` "NewEnumerator7" :`8` "NewEnumerator8" :`9` "NewEnumerator9" :!type "/Game/PROJECT/GRID/E_PositionNumber Enum") _returnvalue)
      (bind _rootcomponent (`Actor.RootComponent` _returnvalue))
      (`SceneComponent.K2_AttachToComponent` _rootcomponent (`self.DefaultSceneRoot`) "None" "KeepRelative" "KeepRelative" "KeepRelative" true)
      (bind _asstatic_mesh_component (cast `StaticMeshComponent` _rootcomponent :!pure true))
      (`PrimitiveComponent.SetMaterial` _asstatic_mesh_component 0 "/Game/PROJECT/GRID/M_squareMaterial.M_squareMaterial")
      (`PrimitiveComponent.SetCollisionEnabled` _asstatic_mesh_component "QueryAndPhysics")
      (`PrimitiveComponent.SetCollisionResponseToAllChannels` _asstatic_mesh_component "ECR_Block")
      (bind _staticmesh (`StaticMeshComponent.StaticMesh` _asstatic_mesh_component))
      (bind _staticmesh_2 (`StaticMeshComponent.StaticMesh` _asstatic_mesh_component))
      (`SceneComponent.K2_SetRelativeLocation` _asstatic_mesh_component (`KismetMathLibrary.MakeVector` (- (* (`KismetMathLibrary.Conv_IntToDouble` _index) (.x (`.BoxExtent` (`KismetMathLibrary.BreakBoxSphereBounds` (`StaticMesh.GetBounds` _staticmesh)))) 2.0) (* (`self.gridWidth`) (.x (`.BoxExtent` (`KismetMathLibrary.BreakBoxSphereBounds` (`StaticMesh.GetBounds` _staticmesh)))))) (- (* (`KismetMathLibrary.Conv_IntToDouble` _index_2) (.x (`.BoxExtent` (`KismetMathLibrary.BreakBoxSphereBounds` (`StaticMesh.GetBounds` _staticmesh_2)))) 2.0) (* (`self.gridHeight`) (.x (`.BoxExtent` (`KismetMathLibrary.BreakBoxSphereBounds` (`StaticMesh.GetBounds` _staticmesh_2))))))) false false))))

(fn `get direction`
  (params (`From Square` :type "/Game/PROJECT/GRID/BP_square Object Reference") (`To Square` :type "/Game/PROJECT/GRID/BP_square Object Reference"))
  (returns (Dir :type "/Game/PROJECT/GRID/E_direction Enum"))
  (bind _squaresarray (`self.squaresArray`))
  (bind _returnvalue (`KismetArrayLibrary.Array_Find` _squaresarray `To Square`))
  (bind _returnvalue_2 (`KismetArrayLibrary.Array_Find` _squaresarray `From Square`))
  (if (== _returnvalue (- _returnvalue_2 10))
    (return "NewEnumerator0")
    (elif (== _returnvalue (+ _returnvalue_2 10))
      (return "NewEnumerator1")
      (elif (== _returnvalue (- _returnvalue_2 1))
        (return "NewEnumerator2")
        (elif (== _returnvalue (+ _returnvalue_2 1))
          (return "NewEnumerator3"))))))

(fn `GetCrossedAdjacentPlaces`
  (params (`From current Square` :type "/Game/PROJECT/GRID/BP_square Object Reference"))
  (returns (Top :type "/Game/PROJECT/GRID/BP_square Object Reference") (Down :type "/Game/PROJECT/GRID/BP_square Object Reference") (Left :type "/Game/PROJECT/GRID/BP_square Object Reference") (Right :type "/Game/PROJECT/GRID/BP_square Object Reference") (AllCrossedAdjacentPlaces :type "Array of /Game/PROJECT/GRID/BP_square Object Reference") (`Top occuped` :type Boolean) (`Down Occupied` :type Boolean) (`Left Occupied` :type Boolean) (`Right Occupied` :type Boolean))
  (locals (AllCrossedAdjacentSquares :type "Map of /Game/PROJECT/GRID/E_direction Enum to /Game/PROJECT/GRID/BP_square Object Reference"))
  (bind _allcrossedadjacentsquares (`local.AllCrossedAdjacentSquares`))
  (bind _returnvalue (`KismetArrayLibrary.Array_Find` (`self.squaresArray`) `From current Square`))
  (bind _output (`|GetArrayItem` (`self.squaresArray`) (+ _returnvalue 1)))
  (bind _output_2 (`|GetArrayItem` (`self.squaresArray`) (- _returnvalue 10)))
  (bind _output_3 (`|GetArrayItem` (`self.squaresArray`) (+ _returnvalue 10)))
  (bind _output_4 (`|GetArrayItem` (`self.squaresArray`) (- _returnvalue 1)))
  (`BlueprintMapLibrary.Map_Add` _allcrossedadjacentsquares "NewEnumerator0" _output_2)
  (`BlueprintMapLibrary.Map_Add` _allcrossedadjacentsquares "NewEnumerator1" _output_3)
  (`BlueprintMapLibrary.Map_Add` _allcrossedadjacentsquares "NewEnumerator2" _output_4)
  (`BlueprintMapLibrary.Map_Add` _allcrossedadjacentsquares "NewEnumerator3" _output)
  (bind _places_adjacent_array1 (`self.RemoveOutsideCrossedAdjacentPlaces` _allcrossedadjacentsquares (`local.From current Square`)))
  (return _output_2 _output_3 _output_4 _output _places_adjacent_array1 (`/Game/PROJECT/GRID/BP_square.occuped` _output_2) (`/Game/PROJECT/GRID/BP_square.occuped` _output_3) (`/Game/PROJECT/GRID/BP_square.occuped` _output_4) (`/Game/PROJECT/GRID/BP_square.occuped` _output)))

(fn `RemoveOutsideCrossedAdjacentPlaces`
  (params (`places adjacent array` :type "Map of /Game/PROJECT/GRID/E_direction Enum to /Game/PROJECT/GRID/BP_square Object Reference") (`occupied place` :type "/Game/PROJECT/GRID/BP_square Object Reference"))
  (returns (`places adjacent array1` :type "Array of /Game/PROJECT/GRID/BP_square Object Reference"))
  (`|ExecutionSequence`
    (:`then_0`
      (if (`|EnumEquality` (`/Game/PROJECT/GRID/BP_square.indexNumber` `occupied place`) "NewEnumerator0")
        (`BlueprintMapLibrary.Map_Remove` `places adjacent array` "NewEnumerator2")))
    (:`then_1`
      (if (`|EnumEquality` (`/Game/PROJECT/GRID/BP_square.indexNumber` `occupied place`) "NewEnumerator9")
        (`BlueprintMapLibrary.Map_Remove` `places adjacent array` "NewEnumerator3")))
    (:`then_2`
      (if (`|EnumEquality` (`/Game/PROJECT/GRID/BP_square.indexLetter` `occupied place`) "NewEnumerator9")
        (`BlueprintMapLibrary.Map_Remove` `places adjacent array` "NewEnumerator1")))
    (:`then_3`
      (if (`|EnumEquality` (`/Game/PROJECT/GRID/BP_square.indexLetter` `occupied place`) "NewEnumerator0")
        (`BlueprintMapLibrary.Map_Remove` `places adjacent array` "NewEnumerator0")))
    (:`then_4`
      (bind _values (`BlueprintMapLibrary.Map_Values` `places adjacent array`))
      (return _values))))

(fn `UserConstructionScript`)